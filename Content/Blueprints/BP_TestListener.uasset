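; BP_TestListener is a test actor that visualizes beat events from the rhythm sequencer on a cylinder.
; On BeginPlay it finds BP_RhythmSequencer, binds to its beat event and reacts only to event names listed in TrackRows.
; Kick plays a timeline that scales the cylinder relative to its initial scale, Snare plays one that adds roll rotation, and Hat flip-flops between black and blue materials.
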(event `self.ReceiveBeginPlay`
  (set `self.InitScale` (`SceneComponent.K2_GetComponentScale` (`self.Cylinder`)))
  (bind _returnvalue (`GameplayStatics.GetActorOfClass` "/Game/Blueprints/BP_RhythmSequencer.BP_RhythmSequencer_C"))
  (add `/Game/Blueprints/BP_RhythmSequencer.OnBeatEvent` _returnvalue (delegate `Beat`)))

(event `Beat`
  (params (EventName :type Name))
  (for _array_element (`self.TrackRows`)
    (if (== EventName _array_element)
      (switch `name` EventName
        (:`Kick`
          (bind (_direction _scaletrack) (`Timeline|Timeline` :!via `PlayFromStart`)
            (:`Update`
              (`SceneComponent.SetWorldScale3D` (`self.Cylinder`) (* (`KismetMathLibrary.Conv_DoubleToVector` _scaletrack) (`self.InitScale`))))))
        (:`Snare`
          (bind (_direction_2 _scaletrack_2) (`Timeline|Timeline_0` :!via `PlayFromStart`)
            (:`Update`
              (`SceneComponent.K2_AddWorldRotation` (`self.Cylinder`) (`KismetMathLibrary.MakeRotator` (* _scaletrack_2 3.0)) false false))))
        (:`Hat`
          (`/Engine/EditorBlueprintResources/StandardMacros.FlipFlop`
            (:`A`
              (`PrimitiveComponent.SetMaterial` (`self.Cylinder`) 0 "/Game/Materials/M_Black.M_Black"))
            (:`B`
              (`PrimitiveComponent.SetMaterial` (`self.Cylinder`) 0 "/Game/Materials/M_Blue.M_Blue"))))))))

(fn `UserConstructionScript`)