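; BP_RhythmSequencer is a step sequencer that plays a looping sound and broadcasts named beat events from pattern data.
; On BeginPlay it starts two independent looping timers: one replays the 2D sound each time its duration elapses, the other ticks at sixteenth-note intervals derived from the pattern's BPM.
; Each tick advances a wrapping beat index and calls OnBeatEvent with the event name of every channel active on that step.
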(event `self.ReceiveBeginPlay`
  (`self.StartSequence`))

(event `Key|F`
  (params (Key :type "Key Structure")))

(fn `OnBeatTick`
  (bind _result (`/Engine/EditorBlueprintResources/StandardMacros.IncrementInt` (`self.CurrentBeat`))
    (:`  `
      (set `self.CurrentBeat` (mod _result (`/Game/Blueprints/BP_ChannelRackData.BeatCount` (`self.PatternData`))))
      (for _array_element (`/Game/Blueprints/BP_ChannelRackData.Channels` (`self.PatternData`))
        (bind (_eventname _activebeats) (break `/Game/Data/S_ChannelData` _array_element))
        (if (`|GetArrayItem` _activebeats (`self.CurrentBeat`))
          (`self.OnBeatEvent` _eventname))))))

(fn `PlaySound`
  (`GameplayStatics.PlaySound2D` (`self.Sound`) 1.0 1.0 0.0 null null))

(fn `StartSequence`
  (`|ExecutionSequence`
    (:`then_0`
      (set `self.CurrentBeat` 0)
      (`self.PlaySound`)
      (`KismetSystemLibrary.K2_SetTimer` null "PlaySound" (`SoundBase.Duration` (`self.Sound`)) true))
    (:`then_1`
      (`KismetSystemLibrary.K2_SetTimer` null "OnBeatTick" (/ 15.0 (`/Game/Blueprints/BP_ChannelRackData.BPM` (`self.PatternData`))) true)
      (`KismetSystemLibrary.PrintString` "Hello"))))

(fn `UserConstructionScript`)